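; BP_Car is a physics vehicle Blueprint that implements raycast suspension, with no driving or steering logic.
; Each Tick, it runs SuspensionCast for the four wheel components, tracing a short distance straight down in world space with debug drawing.
; On a hit, it pushes the Box body upward at that wheel's location, scaling force linearly with compression, like an undamped spring.
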(event `self.ReceiveTick`
  (params (DeltaSeconds :type "Float (single-precision)"))
  (`self.SuspensionCast` (`self.FL_Wheel`))
  (`self.SuspensionCast` (`self.FR_Wheel`))
  (`self.SuspensionCast` (`self.BL_Wheel`))
  (`self.SuspensionCast` (`self.BR_Wheel`)))

(fn `SuspensionCast`
  (params (WheelComp :type "SceneComponent Object Reference"))
  (bind _returnvalue (`SceneComponent.K2_GetComponentLocation` WheelComp))
  (bind _outhit (`KismetSystemLibrary.LineTraceSingle` :`Start` _returnvalue :`End` (+ _returnvalue (0.0 0.0 -60.0)) :`TraceChannel` "TraceTypeQuery1" :`DrawDebugType` "ForOneFrame"))
  (bind (_bblockinghit _binitialoverlap _time _distance _location _impactpoint _normal _impactnormal _physmat _hitactor _hitcomponent _hitbonename _bonename _hititem _elementindex _faceindex _tracestart _traceend) (`GameplayStatics.BreakHitResult` _outhit))
  (if _bblockinghit
    (`PrimitiveComponent.AddForceAtLocation` (`self.Box`) (* (- 1.0 (`KismetMathLibrary.NormalizeToRange` _distance 0.0 60.0)) (`KismetMathLibrary.GetDirectionUnitVector` _traceend _tracestart) 90000.0) (`SceneComponent.K2_GetComponentLocation` (`local.WheelComp`)) "None")))

(fn `UserConstructionScript`)